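; Half-elf female warrior character Blueprint that adds hold-to-run movement.
; The Run input action calls StartRun on press and StopRun on release, switching the CharacterMovement max walk speed between RunSpeed and WalkSpeed.
; The BeginPlay, overlap and Tick events are disabled placeholders, and the construction script only calls its parent.
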(event `InputAction|Run`
  (params (Key :type "Key Structure"))
  (:`Pressed`
    (`self.StartRun`))
  (:`Released`
    (`self.StopRun`)))

(fn `StartRun`
  (set `CharacterMovementComponent.MaxWalkSpeed` (`self.RunSpeed`) (`self.CharacterMovement`)))

(fn `StopRun`
  (set `CharacterMovementComponent.MaxWalkSpeed` (`self.WalkSpeed`) (`self.CharacterMovement`)))

(fn `UserConstructionScript`
  (`parent.UserConstructionScript`))